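; BP_Obstacle is a scrolling obstacle that awards the player a point when passed, apparently for a Dino-style runner.
; On BeginPlay it gets a random integer scale per axis, then moves along negative X by a fixed, frame-rate-dependent step each Tick.
; When BP_MyPawn stops overlapping BoxComponent, it increments GamePoint in BP_DinoGameInstance and prints the score.
; The Box begin-overlap event is empty, so no hit response happens here.
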(event OnComponentBeginOverlap(Box)
  (params (OverlappedComponent :type Primitive%20Component%20Object%20Reference) (OtherActor :type Actor%20Object%20Reference) (OtherComp :type Primitive%20Component%20Object%20Reference) (OtherBodyIndex :type Integer) (bFromSweep :type Boolean) (SweepResult :type Hit%20Result%20Structure%20%28by%20ref%29)))

(event OnComponentEndOverlap(BoxComponent)
  (params (OverlappedComponent :type Primitive%20Component%20Object%20Reference) (OtherActor :type Actor%20Object%20Reference) (OtherComp :type Primitive%20Component%20Object%20Reference) (OtherBodyIndex :type Integer))
  (Utilities|Casting|CastToBP_MyPawn OtherActor)
  (bind _asbp_dino_game_instance (Utilities|Casting|CastToBP_DinoGameInstance (Game|GetGameInstance)))
  (bind _result (Math|Integer|IncrementInt (Variables|/Game/BP_DinoGameInstance.BP_DinoGameInstance_C|GetGamePoint _asbp_dino_game_instance))
    (:%20%20
      (Development|PrintString (Utilities|String|ToString(Integer) _result)))))

(event EventBeginPlay
  (Transformation|SetActorScale3D (Math|Vector|MakeVector (Math|Conversions|ToFloat(Integer) (Math|Random|RandomIntegerinRange 1 3)) (Math|Conversions|ToFloat(Integer) (Math|Random|RandomIntegerinRange 1 3)) (Math|Conversions|ToFloat(Integer) (Math|Random|RandomIntegerinRange 1 3)))))

(event Collision|EventActorBeginOverlap
  (params (OtherActor :type Actor%20Object%20Reference)))

(event EventTick
  (params (DeltaSeconds :type Float%20%28single-precision%29))
  (Transformation|AddActorWorldOffset (Math|Vector|MakeVector -5.0 0.0 0.0)))

(fn ConstructionScript)